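; Chess board actor that spawns a checkered 8x8 tile grid, both sets of pieces and a fixed camera view on BeginPlay.
; Left-click cursor traces select a tagged piece, then move it to an unoccupied tile after a per-type legality check.
; Only pawns register with tiles and have movement rules, with the double-step limited by one board-wide counter.
; Other piece rules are stubs, and capture logic is unfinished and never called.
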(event EventBeginPlay
  (CallFunction|SpawnCamera)
  (CallFunction|SpawnBoard)
  (CallFunction|SpawnPieces)
  (Input|EnableInput (Game|GetPlayerController 0)))

(event Input|MouseEvents|LeftMouseButton
  (params (Key :type Key%20Structure :default "None"))
  (bind _returnvalue (Game|GetPlayerController 0))
  (:Pressed
    (Variables|/Script/Engine.PlayerController|SetbShowMouseCursor _returnvalue true)
    (CallFunction|MovePieces _returnvalue)))

(fn ConstructionScript)

(fn SpawnBoard
  (bind _startlocation (Variables|Default|GetStartLocation))
  (bind _tilesize (Variables|Default|GetTileSize))
  (for _index (range 0 7) ; X (ligne)
    (LocalVariables|SetIndexX _index)
    (for _index_2 (range 0 7) ; Y (colonne)
      (LocalVariables|SetIndexY _index_2)
      ;[0.15 0.15 0.15 0.5] Tile pos calcul + spawn
      (bind _returnvalue (Game|SpawnActorfromClass (Variables|Default|GetTileClass) (Math|Conversions|ToTransform(Vector) (Math|Vector|MakeVector (* (+ (LocalVariables|GetIndexX) (.x _startlocation)) _tilesize) (* (+ (LocalVariables|GetIndexY) (.y _startlocation)) _tilesize) (.z _startlocation))) "Undefined" "MultiplyWithRoot" 0 0))
      (Utilities|Array|Add (Variables|Default|GetTiles) _returnvalue)
      (Variables|/Game/logic/BP_ChessTile.BP_ChessTile_C|SetGridX _returnvalue (LocalVariables|GetIndexX))
      (Variables|/Game/logic/BP_ChessTile.BP_ChessTile_C|SetGridY _returnvalue (LocalVariables|GetIndexY))
      (CallFunction|AreTilesBlackorWhite (LocalVariables|GetIndexX) (LocalVariables|GetIndexY) (Variables|/Game/logic/BP_ChessTile.BP_ChessTile_C|GetCube _returnvalue)))))

(fn AreTilesBlackorWhite
  (params (X :type Integer) (Y :type Integer) (TargetToColor :type Primitive%20Component%20Object%20Reference))
  ;[0.15 0.15 0.15 0.5] Is White or Black
  (if (== (Math|Integer|%(Integer) (+ X Y) 2) 0)
    (Rendering|Material|SetMaterial TargetToColor 0 "/Game/Assets/Black_.Black_")
    (else
      (Rendering|Material|SetMaterial TargetToColor 0 "/Game/Assets/_White_Marble._White_Marble"))))

(fn SpawnCamera
  ;[0.15 0.15 0.15 0.5] Place camera
  (Game|Player|SetViewTargetwithBlend (Game|GetPlayerController 0) self 0.0 "VTBlend_Linear" 0.0 false)
  (Transformation|SetWorldLocationAndRotation (Variables|Default|GetCamera) (Math|Vector|MakeVector 1.5e+02 0.0 8e+02) "-60.000000,90.000000,0.000000" false false))

(fn SpawnPieces
  (for _index (range 0 7) ; x
    (Variables|Default|SetTileIndexX _index)
    (for _index_2 (range 0 7) ; y
      (Variables|Default|SetTileIndexY _index_2)
      ;[0.15 0.15 0.15 0.5] Set current tile and location to spawn
      (bind _output_get (LocalVariables|SetTileIndex (+ _index_2 (* _index 8))))
      (bind _output_get_2 (Variables|Default|SetCurrentTile (Utilities|Array|Get(acopy) (Variables|Default|GetTiles) _output_get)))
      (Variables|Default|SetCurrentLocatio, (Transformation|GetActorLocation _output_get_2))
      (CallFunction|SpawnPawns)
      (CallFunction|SpawnWhitePieces)
      (CallFunction|SpawnBlackPieces))))

(fn SpawnWhitePieces
  (bind _tileindexy (Variables|Default|GetTileIndexY))
  (bind _tileindexy_2 (Variables|Default|GetTileIndexY))
  (bind _tileindexy_3 (Variables|Default|GetTileIndexY))
  (if (== (Variables|Default|GetTileIndexX) 0)
    (if (== (Variables|Default|GetTileIndexY) 4)
      (bind _returnvalue (Game|SpawnActorfromClass "/Game/logic/Pieces/BP_King.BP_King_C" (Math|Conversions|ToTransform(Vector) (Variables|Default|GetCurrentLocatio,)) "Undefined" "MultiplyWithRoot" 0 0))
      (Rendering|Material|SetMaterial (Variables|/Game/logic/Pieces/BP_King.BP_King_C|GetKing _returnvalue) 0 "/Game/Assets/_White_Marble._White_Marble")
      (elif (== (Variables|Default|GetTileIndexY) 3)
        (bind _returnvalue_2 (Game|SpawnActorfromClass "/Game/logic/Pieces/BP_Queen.BP_Queen_C" (Math|Conversions|ToTransform(Vector) (Variables|Default|GetCurrentLocatio,)) "Undefined" "MultiplyWithRoot" 0 0))
        (Rendering|Material|SetMaterial (Variables|/Game/logic/Pieces/BP_Queen.BP_Queen_C|GetQueen _returnvalue_2) 0 "/Game/Assets/_White_Marble._White_Marble")
        (elif (or (== _tileindexy 2) (== _tileindexy 5))
          (bind _returnvalue_3 (Game|SpawnActorfromClass "/Game/logic/Pieces/BP_Bishop.BP_Bishop_C" (Math|Conversions|ToTransform(Vector) (Variables|Default|GetCurrentLocatio,)) "Undefined" "MultiplyWithRoot" 0 0))
          (Rendering|Material|SetMaterial (Variables|/Game/logic/Pieces/BP_Bishop.BP_Bishop_C|GetBishop _returnvalue_3) 0 "/Game/Assets/_White_Marble._White_Marble")
          (elif (or (== _tileindexy_2 1) (== _tileindexy_2 6))
            (bind _returnvalue_4 (Game|SpawnActorfromClass "/Game/logic/Pieces/BP_Knight.BP_Knight_C" (Math|Conversions|ToTransform(Vector) (Variables|Default|GetCurrentLocatio,)) "Undefined" "MultiplyWithRoot" 0 0))
            (Rendering|Material|SetMaterial (Variables|/Game/logic/Pieces/BP_Knight.BP_Knight_C|GetKnight _returnvalue_4) 0 "/Game/Assets/_White_Marble._White_Marble")
            (elif (or (== _tileindexy_3 0) (== _tileindexy_3 7))
              (bind _returnvalue_5 (Game|SpawnActorfromClass "/Game/logic/Pieces/BP_Rook.BP_Rook_C" (Math|Conversions|ToTransform(Vector) (Variables|Default|GetCurrentLocatio,)) "Undefined" "MultiplyWithRoot" 0 0))
              (Rendering|Material|SetMaterial (Variables|/Game/logic/Pieces/BP_Rook.BP_Rook_C|GetRook _returnvalue_5) 0 "/Game/Assets/_White_Marble._White_Marble"))))))))

(fn SpawnBlackPieces
  (bind _tileindexy (Variables|Default|GetTileIndexY))
  (bind _tileindexy_2 (Variables|Default|GetTileIndexY))
  (bind _tileindexy_3 (Variables|Default|GetTileIndexY))
  (if (== (Variables|Default|GetTileIndexX) 7)
    (if (== (Variables|Default|GetTileIndexY) 4)
      (bind _returnvalue (Game|SpawnActorfromClass "/Game/logic/Pieces/BP_King.BP_King_C" (Math|Conversions|ToTransform(Vector) (Variables|Default|GetCurrentLocatio,)) "Undefined" "MultiplyWithRoot" 0 0))
      (Rendering|Material|SetMaterial (Variables|/Game/logic/Pieces/BP_King.BP_King_C|GetKing _returnvalue) 0 "/Game/Assets/Black_Marble.Black_Marble")
      (elif (== (Variables|Default|GetTileIndexY) 3)
        (bind _returnvalue_2 (Game|SpawnActorfromClass "/Game/logic/Pieces/BP_Queen.BP_Queen_C" (Math|Conversions|ToTransform(Vector) (Variables|Default|GetCurrentLocatio,)) "Undefined" "MultiplyWithRoot" 0 0))
        (Rendering|Material|SetMaterial (Variables|/Game/logic/Pieces/BP_Queen.BP_Queen_C|GetQueen _returnvalue_2) 0 "/Game/Assets/Black_Marble.Black_Marble")
        (elif (or (== _tileindexy_3 2) (== _tileindexy_3 5))
          (bind _returnvalue_3 (Game|SpawnActorfromClass "/Game/logic/Pieces/BP_Bishop.BP_Bishop_C" (Math|Conversions|ToTransform(Vector) (Variables|Default|GetCurrentLocatio,)) "Undefined" "MultiplyWithRoot" 0 0))
          (Rendering|Material|SetMaterial (Variables|/Game/logic/Pieces/BP_Bishop.BP_Bishop_C|GetBishop _returnvalue_3) 0 "/Game/Assets/Black_Marble.Black_Marble")
          (elif (or (== _tileindexy 1) (== _tileindexy 6))
            (bind _returnvalue_4 (Game|SpawnActorfromClass "/Game/logic/Pieces/BP_Knight.BP_Knight_C" (Math|Conversions|ToTransform(Vector) (Variables|Default|GetCurrentLocatio,)) "Undefined" "MultiplyWithRoot" 0 0))
            (Rendering|Material|SetMaterial (Variables|/Game/logic/Pieces/BP_Knight.BP_Knight_C|GetKnight _returnvalue_4) 0 "/Game/Assets/Black_Marble.Black_Marble")
            (elif (or (== _tileindexy_2 0) (== _tileindexy_2 7))
              (bind _returnvalue_5 (Game|SpawnActorfromClass "/Game/logic/Pieces/BP_Rook.BP_Rook_C" (Math|Conversions|ToTransform(Vector) (Variables|Default|GetCurrentLocatio,)) "Undefined" "MultiplyWithRoot" 0 0))
              (Rendering|Material|SetMaterial (Variables|/Game/logic/Pieces/BP_Rook.BP_Rook_C|GetRook _returnvalue_5) 0 "/Game/Assets/Black_Marble.Black_Marble"))))))))

(fn SpawnPawns
  (bind _currenttile (Variables|Default|GetCurrentTile))
  (if (== (Variables|Default|GetTileIndexX) 1)
    (bind _returnvalue (Game|SpawnActorfromClass "/Game/logic/Pieces/BP_Pawn.BP_Pawn_C" (Math|Conversions|ToTransform(Vector) (Variables|Default|GetCurrentLocatio,)) "Undefined" "MultiplyWithRoot" 0 0))
    (CallFunction|SetNewTile _returnvalue)
    (Rendering|Material|SetMaterial (Variables|/Game/logic/Pieces/BP_Pawn.BP_Pawn_C|GetPawn _returnvalue) 0 "/Game/Assets/_White_Marble._White_Marble")
    (Variables|/Game/logic/BP_ChessTile.BP_ChessTile_C|SetIsOccupied (Variables|Default|GetCurrentTile) true)
    (Variables|/Game/logic/Pieces/BP_ChessPiece.BP_ChessPiece_C|SetisWhite _returnvalue true)
    (Variables|/Game/logic/BP_ChessTile.BP_ChessTile_C|SetGridX _currenttile (Variables|Default|GetTileIndexX))
    (Variables|/Game/logic/BP_ChessTile.BP_ChessTile_C|SetGridY _currenttile (Variables|Default|GetTileIndexY))
    (Variables|/Game/logic/BP_ChessTile.BP_ChessTile_C|SetCurrentPiece _currenttile _returnvalue)
    (elif (== (Variables|Default|GetTileIndexX) 6)
      (bind _returnvalue_2 (Game|SpawnActorfromClass "/Game/logic/Pieces/BP_Pawn.BP_Pawn_C" (Math|Conversions|ToTransform(Vector) (Variables|Default|GetCurrentLocatio,)) "Undefined" "MultiplyWithRoot" 0 0))
      (CallFunction|SetNewTile _returnvalue_2)
      (Rendering|Material|SetMaterial (Variables|/Game/logic/Pieces/BP_Pawn.BP_Pawn_C|GetPawn _returnvalue_2) 0 "/Game/Assets/Black_Marble.Black_Marble")
      (Variables|/Game/logic/BP_ChessTile.BP_ChessTile_C|SetIsOccupied (Variables|Default|GetCurrentTile) true)
      (Variables|/Game/logic/Pieces/BP_ChessPiece.BP_ChessPiece_C|SetisWhite _returnvalue_2 false))))

(fn MovePieces
  (params (PlayerController :type Player%20Controller%20Object%20Reference))
  (bind _hitresult (Game|Player|GetHitResultUnderCursorbyChannel PlayerController "TraceTypeQuery1" true))
  (bind _hitactor (Collision|BreakHitResult _hitresult))
  ;[0.15 0.15 0.15 0.5] Select piece logic
  (if (Actor|ActorHasTag _hitactor "Piece")
    (bind _asbp_chess_piece (Utilities|Casting|CastToBP_ChessPiece _hitactor))
    (Variables|Default|SetSelectedPiece _asbp_chess_piece)
    (else
      ;[0.15 0.15 0.15 0.5] Is Actor a Tile and a piece is selected
      (if (and (Actor|ActorHasTag _hitactor "Tile") (Utilities|IsValid (Variables|Default|GetSelectedPiece)))
        ;[0.15 0.15 0.15 0.5] Is Tile occupied
        (bind _asbp_chess_tile (Utilities|Casting|CastToBP_ChessTile _hitactor))
        (bind _output_get (LocalVariables|SetSelectedTileCasted _asbp_chess_tile))
        (if (not (Variables|/Game/logic/BP_ChessTile.BP_ChessTile_C|GetIsOccupied _asbp_chess_tile))
          ;[0.15 0.15 0.15 0.5] Is Move allowed
          (bind _allowed (CallFunction|IsMoveLegal (Variables|Default|GetSelectedPiece) _output_get))
          (if _allowed
            (CallFunction|MoveandReplaceOld (Transformation|GetActorLocation _asbp_chess_tile) (LocalVariables|GetSelectedTileCasted))))))))

(fn SetNewTile
  (params (SpawnReturn :type BP%20Chess%20Piece%20Object%20Reference))
  (bind _output_get (Variables|/Game/logic/Pieces/BP_ChessPiece.BP_ChessPiece_C|SetCurrentTile SpawnReturn (Variables|Default|GetCurrentTile)))
  (Transformation|SetActorLocation SpawnReturn (Transformation|GetActorLocation _output_get) false false))

(fn IsMoveLegal
  (params (Piece :type BP%20Chess%20Piece%20Object%20Reference) (TargetTile :type BP%20Chess%20Tile%20Object%20Reference))
  (bind _currenttile (Variables|Default|GetCurrentTile))
  ;[0.15 0.15 0.15 0.5] Setting target and initial position in array
  (Variables|Default|SetTileIndexX (Variables|/Game/logic/BP_ChessTile.BP_ChessTile_C|GetGridX _currenttile))
  (Variables|Default|SetTileIndexY (Variables|/Game/logic/BP_ChessTile.BP_ChessTile_C|GetGridY _currenttile))
  (LocalVariables|SetTargetX (Variables|/Game/logic/BP_ChessTile.BP_ChessTile_C|GetGridX TargetTile))
  (LocalVariables|SetTargetY (Variables|/Game/logic/BP_ChessTile.BP_ChessTile_C|GetGridY TargetTile))
  (bind _asbp_pawn (Utilities|Casting|CastToBP_Pawn Piece)
    (:then
      (bind _ispawnallowedtomove (CallFunction|IsMoveLegalPawn _asbp_pawn (LocalVariables|GetTargetX) (LocalVariables|GetTargetY)))
      (LocalVariables|SetisAllowed _ispawnallowedtomove))
    (:CastFailed
      (bind _asbp_rook (Utilities|Casting|CastToBP_Rook Piece)
        (:then
          (bind _is_rook_allowed_to_move (CallFunction|IsMoveLegalRook _asbp_rook (LocalVariables|GetTargetX) (LocalVariables|GetTargetY)))
          (LocalVariables|SetisAllowed _is_rook_allowed_to_move))
        (:CastFailed
          (bind _asbp_bishop (Utilities|Casting|CastToBP_Bishop Piece)
            (:then
              (bind _isbishopallowedtomove (CallFunction|IsMoveLegalBishop _asbp_bishop (LocalVariables|GetTargetX) (LocalVariables|GetTargetY)))
              (LocalVariables|SetisAllowed _isbishopallowedtomove))
            (:CastFailed
              (bind _asbp_king (Utilities|Casting|CastToBP_King Piece)
                (:then
                  (bind _iskingallowedtomove (CallFunction|IsMoveLegalKing _asbp_king (LocalVariables|GetTargetX) (LocalVariables|GetTargetY)))
                  (LocalVariables|SetisAllowed _iskingallowedtomove))
                (:CastFailed
                  (bind _asbp_knight (Utilities|Casting|CastToBP_Knight Piece)
                    (:then
                      (bind _isknightallowedtomove (CallFunction|IsMoveLegalKnight _asbp_knight (LocalVariables|GetTargetX) (LocalVariables|GetTargetY)))
                      (LocalVariables|SetisAllowed _isknightallowedtomove))
                    (:CastFailed
                      (bind _asbp_queen (Utilities|Casting|CastToBP_Queen Piece))
                      (bind _isqueenallowedtomove (CallFunction|IsMoveLegalQueen _asbp_queen (LocalVariables|GetTargetX) (LocalVariables|GetTargetY)))
                      (LocalVariables|SetisAllowed _isqueenallowedtomove)))))))))))
  (return (LocalVariables|GetisAllowed)))

(fn IsMoveLegalPawn
  (params (CurrentPawn :type BP%20Pawn%20Object%20Reference) (TargetX :type Integer) (TargetY :type Integer))
  (bind _currenttile (Variables|/Game/logic/Pieces/BP_ChessPiece.BP_ChessPiece_C|GetCurrentTile CurrentPawn))
  ;[0.15 0.15 0.15 0.5] Set X Y then is Pawn white
  (LocalVariables|SetcurrentX (Variables|/Game/logic/BP_ChessTile.BP_ChessTile_C|GetGridX _currenttile))
  (LocalVariables|SetcurrentY (Variables|/Game/logic/BP_ChessTile.BP_ChessTile_C|GetGridY _currenttile))
  (LocalVariables|SetTargetXPawn TargetX)
  (LocalVariables|SetTargetYPawn TargetY)
  (if (Variables|/Game/logic/Pieces/BP_ChessPiece.BP_ChessPiece_C|GetisWhite CurrentPawn)
    (if (and (== 1 (LocalVariables|GetcurrentX)) (< (LocalVariables|GetFirstTimeCounter) 1))
      ;[0.15 0.15 0.15 0.5] counter to avoid 2 moves when on x==1
      (LocalVariables|SetFirstTimeCounter (+ (LocalVariables|GetFirstTimeCounter) 1))
      (LocalVariables|SetcanPawnMove (and (or (== (+ (LocalVariables|GetcurrentX) 1) (LocalVariables|GetTargetXPawn)) (== (+ (LocalVariables|GetcurrentX) 2) (LocalVariables|GetTargetXPawn))) (== (LocalVariables|GetcurrentY) (LocalVariables|GetTargetYPawn))))
      (else
        (LocalVariables|SetcanPawnMove (and (== (+ (LocalVariables|GetcurrentX) 1) (LocalVariables|GetTargetXPawn)) (== (LocalVariables|GetcurrentY) (LocalVariables|GetTargetYPawn))))))
    (elif (and (== 6 (LocalVariables|GetcurrentX)) (< (LocalVariables|GetFirstTimeCounter) 1))
      ;[0.15 0.15 0.15 0.5] counter to avoid 2 moves when on x==6
      (LocalVariables|SetFirstTimeCounter (+ (LocalVariables|GetFirstTimeCounter) 1))
      (LocalVariables|SetcanPawnMove (and (or (== (- (LocalVariables|GetcurrentX) 1) (LocalVariables|GetTargetXPawn)) (== (- (LocalVariables|GetcurrentX) 2) (LocalVariables|GetTargetXPawn))) (== (LocalVariables|GetcurrentY) (LocalVariables|GetTargetYPawn))))
      (else
        (LocalVariables|SetcanPawnMove (and (== (- (LocalVariables|GetcurrentX) 1) (LocalVariables|GetTargetXPawn)) (== (LocalVariables|GetcurrentY) (LocalVariables|GetTargetYPawn)))))))
  (return (LocalVariables|GetcanPawnMove)))

(fn IsMoveLegalKnight
  (params (CurrentKnight :type BP%20Knight%20Object%20Reference) (TargetX :type Integer) (TargetY :type Integer))
  (bind _currenttile (Variables|/Game/logic/Pieces/BP_ChessPiece.BP_ChessPiece_C|GetCurrentTile CurrentKnight))
  ;[0.15 0.15 0.15 0.5] Set X Y then is Knight white
  (LocalVariables|SetCurrentX (Variables|/Game/logic/BP_ChessTile.BP_ChessTile_C|GetGridX _currenttile))
  (LocalVariables|SetCurrentY (Variables|/Game/logic/BP_ChessTile.BP_ChessTile_C|GetGridY _currenttile))
  (LocalVariables|SetTargetXKnight TargetX)
  (LocalVariables|SetTargetYKnight TargetY)
  (if (Variables|/Game/logic/Pieces/BP_ChessPiece.BP_ChessPiece_C|GetisWhite CurrentKnight)
    (if true
      _)
    (elif true
      _)))

(fn IsMoveLegalRook
  (params (current%20Rook :type BP%20Rook%20Object%20Reference) (TargetX :type Integer) (TargetY :type Integer))
  (return false))

(fn IsMoveLegalBishop
  (params (CurrentBishop :type BP%20Bishop%20Object%20Reference) (TagetX :type Integer) (TargetY :type Integer))
  (return false))

(fn IsMoveLegalKing
  (params (CurrentKing :type BP%20King%20Object%20Reference) (TargetX :type Integer) (TargetY :type Integer))
  (return false))

(fn IsMoveLegalQueen
  (params (CurrentQueen :type BP%20Queen%20Object%20Reference) (TargetX :type Integer) (TargetY :type Integer))
  (return false))

(fn CanCapture
  (params (CurrentTile :type BP%20Chess%20Tile%20Object%20Reference))
  (bind _output_get (LocalVariables|SetTargetPiece (Variables|/Game/logic/BP_ChessTile.BP_ChessTile_C|GetCurrentPiece CurrentTile)))
  ;[0.15 0.15 0.15 0.5] Player is white by default
  (if (not (Variables|/Game/logic/Pieces/BP_ChessPiece.BP_ChessPiece_C|GetisWhite _output_get))
    (bind _asbp_pawn (Utilities|Casting|CastToBP_Pawn (LocalVariables|GetTargetPiece)))
    (bind _pawnisallowedtocapture (CallFunction|CanCapturePawn _asbp_pawn))
    (if _pawnisallowedtocapture
      (Actor|DestroyActor (LocalVariables|GetTargetPiece))
      (CallFunction|MoveandReplaceOld (Transformation|GetActorLocation CurrentTile) CurrentTile))))

(fn CanCapturePawn
  (params (TargetPiece :type BP%20Pawn%20Object%20Reference))
  (return false))

(fn MoveandReplaceOld
  (params (ActorLocation :type Vector) (TargetTile :type BP%20Chess%20Tile%20Object%20Reference))
  ;[0.15 0.15 0.15 0.5] Free previous tile & occupy next one
  (Variables|/Game/logic/BP_ChessTile.BP_ChessTile_C|SetIsOccupied (Variables|/Game/logic/Pieces/BP_ChessPiece.BP_ChessPiece_C|GetCurrentTile (Variables|Default|GetSelectedPiece)) false)
  (Transformation|SetActorLocation (Variables|Default|GetSelectedPiece) ActorLocation false false)
  (Variables|/Game/logic/BP_ChessTile.BP_ChessTile_C|SetIsOccupied TargetTile true)
  (Variables|/Game/logic/Pieces/BP_ChessPiece.BP_ChessPiece_C|SetCurrentTile (Variables|Default|GetSelectedPiece) TargetTile)
  (Variables|Default|SetSelectedPiece 0))